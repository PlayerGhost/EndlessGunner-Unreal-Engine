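; EnemyActor_BP is an enemy actor, apparently for a 2D side scroller, that moves along world X at Speed every tick without sweeping.
; It destroys itself when its capsule overlaps a component tagged MapLimit.
; EnemyDamage subtracts from EnemyHealth, then either destroys the actor or prints the remaining health.
; StopEvent zeroes Speed, but its binding to the game mode's GameEnded dispatcher is disconnected and never runs.
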(event OnComponentBeginOverlap(Capsule)
  (params (OverlappedComponent :type Primitive%20Component%20Object%20Reference) (OtherActor :type Actor%20Object%20Reference) (OtherComp :type Primitive%20Component%20Object%20Reference) (OtherBodyIndex :type Integer) (bFromSweep :type Boolean) (SweepResult :type Hit%20Result%20Structure%20%28by%20ref%29))
  (if (Components|ComponentHasTag OtherComp "MapLimit")
    (Actor|DestroyActor)))

(event Custom|EnemyDamage
  (params (DamageTaken :type Integer))
  (bind _output_get (Variables|Default|SetEnemyHealth (- (Variables|Default|GetEnemyHealth) DamageTaken)))
  (if (<= _output_get 0)
    (Actor|DestroyActor)
    (else
      (Development|PrintString "Enemy Health: ")
      (Development|PrintString (Utilities|String|ToString(Integer) (Variables|Default|GetEnemyHealth))))))

(event Custom|StopEvent
  (Variables|Default|SetSpeed 0.0))

(event EventBeginPlay)

(event EventTick
  (params (DeltaSeconds :type Float%20%28single-precision%29))
  (Transformation|AddActorWorldOffset (Math|Vector|MakeVector (* DeltaSeconds (Variables|Default|GetSpeed)) 0.0 0.0)))

(fn ConstructionScript)