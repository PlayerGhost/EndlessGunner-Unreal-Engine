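; Side-scroller boss enemy that chases the player along X, dash-attacks at close range and opens the Win level when its health runs out.
; Tick drives everything from signed X distance: stepped movement, yaw facing, launch-based dashes, flipbook updates and the death check.
; BossDamage lowers health, while capsule overlap directly reduces player health.
; Fire spawns enemy bullets but is never called here, StopEvent is empty, and Atacking is never reset.
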(event OnComponentBeginOverlap(Capsule)
  (params (OverlappedComponent :type Primitive%20Component%20Object%20Reference) (OtherActor :type Actor%20Object%20Reference) (OtherComp :type Primitive%20Component%20Object%20Reference) (OtherBodyIndex :type Integer) (bFromSweep :type Boolean) (SweepResult :type Hit%20Result%20Structure%20%28by%20ref%29))
  (if (Components|ComponentHasTag OtherComp "Player")
    (bind _as2dside_scroller_character (Utilities|Casting|CastTo2DSideScrollerCharacter OtherActor))
    (Variables|/Game/Blueprints/2DSideScrollerCharacter.2DSideScrollerCharacter_C|SetPlayerHealth _as2dside_scroller_character (- (Variables|/Game/Blueprints/2DSideScrollerCharacter.2DSideScrollerCharacter_C|GetPlayerHealth _as2dside_scroller_character) 1e+01))))

(event Custom|BossDamage
  (params (DamageTaken :type Integer))
  (bind _output_get (Variables|Default|SetEnemyHealth (- (Variables|Default|GetEnemyHealth) DamageTaken)))
  (Development|PrintString (Utilities|String|ToString(Integer) _output_get))
  (if (<= _output_get 0)
    (Class|NavMovementComponent|StopActiveMovement (Variables|Character|GetCharacterMovement))))

(event Custom|StopEvent)

(event EventBeginPlay)

(event EventTick
  (params (DeltaSeconds :type Float%20%28single-precision%29))
  (bind _returnvalue (Transformation|GetActorLocation))
  (Utilities|FlowControl|Sequence
    (:then_0
      (bind _output_get (Variables|Default|SetDistance (- (.x (Transformation|GetWorldLocation (Variables|Default|GetCapsule))) (.x (Transformation|GetActorLocation (Game|GetPlayerCharacter 0))))))
      (Utilities|FlowControl|Sequence
        (:then_0
          (if (Math|Float|InRange(Float) _output_get 0.0 2e+02)
            (CallFunction|DashAtack)
            (Utilities|FlowControl|Delay 2.0)
            (Sprite|SetFlipbook (Variables|Default|GetSprite) "/Game/Assets/Sprites/Boss/WalkOn/BossWalkON.BossWalkON")))
        (:then_1
          (if (Math|Float|InRange(Float) _output_get -2e+02 0.0)
            (CallFunction|DashAtack)
            (Utilities|FlowControl|Delay 2.0)
            (Sprite|SetFlipbook (Variables|Default|GetSprite) "/Game/Assets/Sprites/Boss/WalkOn/BossWalkON.BossWalkON")))))
    (:then_1
      (bind _as2dside_scroller_game_mode (Utilities|Casting|CastTo2DSideScrollerGameMode (Game|GetGameMode)))
      (EventDispatchers|AssignGameEndedDispatcher _as2dside_scroller_game_mode (delegate Custom|StopEvent)))
    (:then_2
      (Transformation|SetActorRotation (Math|Rotator|MakeRotator 0.0 0.0 (.yaw (Math|Rotator|FindLookatRotation (Transformation|GetActorLocation (Game|GetPlayerCharacter 0)) (Transformation|GetActorLocation))))))
    (:then_3
      (Variables|Default|SetActorLocation (Math|Vector|MakeVector (.x _returnvalue) (.y _returnvalue) (.z _returnvalue))))
    (:then_4
      (if (Math|Float|InRange(Float) (Variables|Default|GetDistance) 0.0 2.86e+03)
        (Utilities|FlowControl|Delay 0.01)
        (Transformation|SetActorLocation (Math|Vector|MakeVector (- (.x (Variables|Default|GetActorLocation)) 4.0) (.y (Variables|Default|GetActorLocation)) (.z (Variables|Default|GetActorLocation))) false false)
        (Variables|Default|SetMovingLeft true)
        (else
          (Variables|Default|SetMovingLeft false))))
    (:then_5
      (if (Math|Float|InRange(Float) (Variables|Default|GetDistance) -2.86e+03 0.0)
        (Utilities|FlowControl|Delay 0.01)
        (Transformation|SetActorLocation (Math|Vector|MakeVector (+ (.x (Variables|Default|GetActorLocation)) 4.0) (.y (Variables|Default|GetActorLocation)) (.z (Variables|Default|GetActorLocation))) false false)
        (Variables|Default|SetMovingRight true)
        (else
          (Variables|Default|SetMovingRight false))))
    (:then_6
      (CallFunction|UpdateAnimation))
    (:then_7
      (if (<= (Variables|Default|GetEnemyHealth) 0)
        (Game|OpenLevel(byName) "Win")))))

(fn ConstructionScript)

(fn DashAtack
  (Variables|Default|SetAtacking true)
  (Sprite|SetFlipbook (Variables|Default|GetSprite) "/Game/Assets/Sprites/Boss/Dash/BossDash.BossDash")
  (if true
    (Character|LaunchCharacter (+ (Transformation|GetActorUpVector) (* (Transformation|GetActorForwardVector) -2e+02)) true true)))

(fn Fire
  (bind _returnvalue (Game|SpawnActorfromClass "/Game/Blueprints/BulletActor_BP.BulletActor_BP_C" (Transformation|GetWorldTransform (Variables|Default|GetArrow1)) "Undefined" 0 0))
  (Variables|/Game/Blueprints/BulletActor_BP.BulletActor_BP_C|SetEnemyFired _returnvalue true))

(fn UpdateAnimation
  (if (not (Variables|Default|GetAtacking))
    (Sprite|SetFlipbook (Variables|Default|GetSprite) (select (or (Variables|Default|GetMovingLeft) (Variables|Default|GetMovingRight)) "/Game/Assets/Sprites/Boss/WalkOn/BossWalkON.BossWalkON" "/Game/Assets/Sprites/Boss/BossIdle.BossIdle"))))