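; Enemy spawner actor for a 2D side-scroller that periodically spawns enemies ahead of the player while a game is running.
; On BeginPlay it binds Start and Stop to the game mode's game-started and game-ended dispatchers.
; Start spawns once, then runs a looping timer at SpawnInterval, which Stop clears.
; Each spawn places EnemyTemplate at a fixed X offset from the player's location, with fixed Y and Z.
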(event Custom|StartEvent
  (CallFunction|Start))

(event Custom|StopEvent
  (CallFunction|Stop))

(event EventBeginPlay
  (bind _as2dside_scroller_game_mode (Utilities|Casting|CastTo2DSideScrollerGameMode (Game|GetGameMode)))
  (EventDispatchers|BindEventtoGameStartedDispatcher _as2dside_scroller_game_mode (delegate Custom|StartEvent))
  (EventDispatchers|BindEventtoGameEndedDispatcher _as2dside_scroller_game_mode (delegate Custom|StopEvent)))

(event Collision|EventActorBeginOverlap
  (params (OtherActor :type Actor%20Object%20Reference)))

(event EventTick
  (params (DeltaSeconds :type Float%20%28single-precision%29)))

(fn ConstructionScript)

(fn Start
  (CallFunction|Spawn)
  (bind _returnvalue (Utilities|Time|SetTimerbyFunctionName 0 "Spawn" (Variables|Default|GetSpawnInterval) true))
  (Variables|Default|SetTimerHandle _returnvalue))

(fn Stop
  (Utilities|Time|ClearandInvalidateTimerbyHandle (Variables|Default|GetTimerHandle)))

(fn Spawn
  (bind _returnvalue (Actor|GetActorOfClass (Variables|Default|GetPlayerObject)))
  (Game|SpawnActorfromClass (Variables|Default|GetEnemyTemplate) (Math|Transform|MakeTransform (Math|Vector|MakeVector (+ (.X (Math|Vector|BreakVector (Variables|/Game/Blueprints/2DSideScrollerCharacter.2DSideScrollerCharacter_C|GetPlayerLocation _returnvalue))) 1.21e+03) 6e+01 -1.9e+02)) "Undefined" 0 0))