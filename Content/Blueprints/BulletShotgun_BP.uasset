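; BulletShotgun_BP is a shotgun bullet actor that damages enemies and bosses it overlaps, then destroys itself.
; On overlap it checks actor tags: Enemy hits require PlayerFired and cast to either of two enemy Blueprint classes to call EnemyDamage.
; Boss hits call BossDamage with the same fixed damage but skip the PlayerFired check.
; Overlapping a MapLimit-tagged actor also destroys the bullet.
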(event EventBeginPlay)

(event EventTick
  (params (DeltaSeconds :type Float%20%28single-precision%29)))

(event Collision|EventActorBeginOverlap
  (params (OtherActor :type Actor%20Object%20Reference))
  (Variables|Default|SetOtherActor OtherActor)
  (Utilities|FlowControl|Sequence
    (:then_0
      (if (Actor|ActorHasTag OtherActor "Enemy")
        (if (Variables|Default|GetPlayerFired)
          (bind _asenemy_actor_bp (Utilities|Casting|CastToEnemyActor_BP (Variables|Default|GetOtherActor))
            (:then
              (Default|EnemyDamage _asenemy_actor_bp 40)
              (Actor|DestroyActor))
            (:CastFailed
              (bind _asenemy_actor_bp1 (Utilities|Casting|CastToEnemyActor_BP1 (Variables|Default|GetOtherActor)))
              (Default|EnemyDamage _asenemy_actor_bp1 40)
              (Actor|DestroyActor))))))
    (:then_1
      (if (Actor|ActorHasTag OtherActor "Boss")
        (bind _asboss_enemy_actor_bp (Utilities|Casting|CastToBossEnemyActor_BP (Variables|Default|GetOtherActor)))
        (Default|BossDamage _asboss_enemy_actor_bp 40)
        (Actor|DestroyActor)))
    (:then_2
      (if (Actor|ActorHasTag OtherActor "MapLimit")
        (Actor|DestroyActor)))))

(fn ConstructionScript)